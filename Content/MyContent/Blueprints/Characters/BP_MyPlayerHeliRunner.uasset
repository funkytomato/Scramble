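; Player character for a helicopter-style runner, flown by physics thrust and able to shoot projectiles.
; Enhanced Input actions push the collider up, down, left or right while boosting the Niagara trail and thruster audio, and the shoot action spawns BP_BaseProjectile.
; Tick tilts the actor from its vertical velocity, with movement and shooting gated by CanMove.
; Physics simulation is enabled in LevelStarted so the player doesn't fall before play begins.
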(event EventBeginPlay
  (bind _returnvalue (Game|GetPlayerController 0))
  (|CallParentFunction)
  (Utilities|IsValid _returnvalue
    (:Is%20Valid
      (Input|AddMappingContext (PlayerController|LocalPlayerSubsystems|GetEnhancedInputLocalPlayerSubsystem _returnvalue) "/Game/MyContent/Input/ScrambleInputMapping.ScrambleInputMapping" 0 "(bIgnoreAllPressedKeysUntilRelease=True,bForceImmediately=False)"))))

(event EventTick
  (params (DeltaSeconds :type Float%20%28single-precision%29))
  (bind _returnvalue (Transformation|GetVelocity))
  (if (and (CallFunction|CanMove) (Utilities|IsValid self))
    ;[0 0 0] Set actor rotation based on velocity to point in the direction the player is moving.
    (Transformation|SetActorRotation (Math|Rotator|MakeRotator (* (.z _returnvalue) (Variables|Default|GetRollRotationSpeed)) (* (.z _returnvalue) (Variables|Default|GetYawRotationSpeed)) 0.0) true)))

(event Input|EnhancedActionEvents|EnhancedInputActionRightAction
  (params (ActionValue :type Boolean) (ElapsedSeconds :type Float%20%28double-precision%29) (TriggeredSeconds :type Float%20%28double-precision%29) (InputAction :type Input%20Action%20Object%20Reference :default "/Game/MyContent/Input/Actions/RightAction.RightAction"))
  (:Triggered
    (if (CallFunction|CanMove)
      ;[0 0 0] Toggle bTouched to be used on EventTick
      (Variables|Default|SetbTouched true)
      ;[0 0 0] Visual effect for the  particle trail to increase/decrease the scale to simulate a thruster effect
      (Niagara|SetNiagaraVariable(Float) (Variables|Default|GetNiagaraTrail) "SizeMult" 3.0)
      (Niagara|SetNiagaraVariable(Float) (Variables|Default|GetNiagaraTrail) "ForceMult" 1.5)
      ;[0 0 0] Play thruster audio component when pressed and disable it when released
      (Components|Activation|SetActive (Variables|Default|GetThrusterAudio) true false)
      ;[0 0 0] Add Force vertically
      (Physics|AddForce (Variables|Default|GetCharacterCollider) "2000.000000,0.000000,0.000000" "None" true)))
  (:Completed
    (if (CallFunction|CanMove)
      (Variables|Default|SetbTouched false)
      (Niagara|SetNiagaraVariable(Float) (Variables|Default|GetNiagaraTrail) "SizeMult" 1.0)
      (Niagara|SetNiagaraVariable(Float) (Variables|Default|GetNiagaraTrail) "ForceMult" 1.0)
      (Components|Activation|SetActive (Variables|Default|GetThrusterAudio) false true))))

(event Input|EnhancedActionEvents|EnhancedInputActionLeftAction
  (params (ActionValue :type Boolean) (ElapsedSeconds :type Float%20%28double-precision%29) (TriggeredSeconds :type Float%20%28double-precision%29) (InputAction :type Input%20Action%20Object%20Reference :default "/Game/MyContent/Input/Actions/LeftAction.LeftAction"))
  (:Triggered
    (if (CallFunction|CanMove)
      ;[0 0 0] Toggle bTouched to be used on EventTick
      (Variables|Default|SetbTouched true)
      ;[0 0 0] Visual effect for the  particle trail to increase/decrease the scale to simulate a thruster effect
      (Niagara|SetNiagaraVariable(Float) (Variables|Default|GetNiagaraTrail) "SizeMult" 3.0)
      (Niagara|SetNiagaraVariable(Float) (Variables|Default|GetNiagaraTrail) "ForceMult" 1.5)
      ;[0 0 0] Play thruster audio component when pressed and disable it when released
      (Components|Activation|SetActive (Variables|Default|GetThrusterAudio) true false)
      ;[0 0 0] Add Force vertically
      (Physics|AddForce (Variables|Default|GetCharacterCollider) "-2000.000000,0.000000,0.000000" "None" true)))
  (:Completed
    (if (CallFunction|CanMove)
      (Variables|Default|SetbTouched false)
      (Niagara|SetNiagaraVariable(Float) (Variables|Default|GetNiagaraTrail) "SizeMult" 1.0)
      (Niagara|SetNiagaraVariable(Float) (Variables|Default|GetNiagaraTrail) "ForceMult" 1.0)
      (Components|Activation|SetActive (Variables|Default|GetThrusterAudio) false true))))

(event Input|EnhancedActionEvents|EnhancedInputActionUpAction
  (params (ActionValue :type Boolean) (ElapsedSeconds :type Float%20%28double-precision%29) (TriggeredSeconds :type Float%20%28double-precision%29) (InputAction :type Input%20Action%20Object%20Reference :default "/Game/MyContent/Input/Actions/UpAction.UpAction"))
  (:Triggered
    (if (CallFunction|CanMove)
      ;[0 0 0] Toggle bTouched to be used on EventTick
      (Variables|Default|SetbTouched true)
      ;[0 0 0] Visual effect for the  particle trail to increase/decrease the scale to simulate a thruster effect
      (Niagara|SetNiagaraVariable(Float) (Variables|Default|GetNiagaraTrail) "SizeMult" 3.0)
      (Niagara|SetNiagaraVariable(Float) (Variables|Default|GetNiagaraTrail) "ForceMult" 1.5)
      ;[0 0 0] Play thruster audio component when pressed and disable it when released
      (Components|Activation|SetActive (Variables|Default|GetThrusterAudio) true false)
      ;[0 0 0] Add Force vertically
      (Physics|AddForce (Variables|Default|GetCharacterCollider) "0, 0,2000.000000" "None" true)))
  (:Completed
    (if (CallFunction|CanMove)
      (Variables|Default|SetbTouched false)
      (Niagara|SetNiagaraVariable(Float) (Variables|Default|GetNiagaraTrail) "SizeMult" 1.0)
      (Niagara|SetNiagaraVariable(Float) (Variables|Default|GetNiagaraTrail) "ForceMult" 1.0)
      (Components|Activation|SetActive (Variables|Default|GetThrusterAudio) false true))))

(event Input|EnhancedActionEvents|EnhancedInputActionDownAction
  (params (ActionValue :type Boolean) (ElapsedSeconds :type Float%20%28double-precision%29) (TriggeredSeconds :type Float%20%28double-precision%29) (InputAction :type Input%20Action%20Object%20Reference :default "/Game/MyContent/Input/Actions/DownAction.DownAction"))
  (:Triggered
    (if (CallFunction|CanMove)
      ;[0 0 0] Toggle bTouched to be used on EventTick
      (Variables|Default|SetbTouched true)
      ;[0 0 0] Visual effect for the  particle trail to increase/decrease the scale to simulate a thruster effect
      (Niagara|SetNiagaraVariable(Float) (Variables|Default|GetNiagaraTrail) "SizeMult" 3.0)
      (Niagara|SetNiagaraVariable(Float) (Variables|Default|GetNiagaraTrail) "ForceMult" 1.5)
      ;[0 0 0] Play thruster audio component when pressed and disable it when released
      (Components|Activation|SetActive (Variables|Default|GetThrusterAudio) true false)
      ;[0 0 0] Add Force vertically
      (Physics|AddForce (Variables|Default|GetCharacterCollider) "0.000000,0.000000,-2000.000000" "None" true)))
  (:Completed
    (if (CallFunction|CanMove)
      (Variables|Default|SetbTouched false)
      (Niagara|SetNiagaraVariable(Float) (Variables|Default|GetNiagaraTrail) "SizeMult" 1.0)
      (Niagara|SetNiagaraVariable(Float) (Variables|Default|GetNiagaraTrail) "ForceMult" 1.0)
      (Components|Activation|SetActive (Variables|Default|GetThrusterAudio) false true))))

(event Input|EnhancedActionEvents|EnhancedInputActionShootAction
  (params (ActionValue :type Boolean) (ElapsedSeconds :type Float%20%28double-precision%29) (TriggeredSeconds :type Float%20%28double-precision%29) (InputAction :type Input%20Action%20Object%20Reference :default "/Game/MyContent/Input/Actions/ShootAction.ShootAction"))
  (:Triggered
    (if (CallFunction|CanMove)
      ;[0 0 0] Toggle bTouched to be used on EventTick
      (Variables|Default|SetbTouched true)
      (Audio|SpawnSound2D (Variables|Default|GetShootSound) 1.0 1.0 0.0 0)
      (CallFunction|SpawnProjectile)))
  (:Completed
    (if (CallFunction|CanMove)
      (Variables|Default|SetbTouched false))))

(event Input|ActionEvents|InputActionTouchAction
  (params (Key :type Key%20Structure :default "None"))
  ;[0 0 0] Touch screen and Desktop Input.
)

(fn ConstructionScript
  (|CallParentFunction))

(fn LevelStarted
  (|CallParentFunction)
  ;[0 0 0] Physics starts disabled to stop the player falling whilst paused or during level start delay. Enable physics here when the game begins.
  (Physics|SetSimulatePhysics (Variables|Default|GetCharacterCollider) true))

(fn SpawnProjectile
  (Game|SpawnActorfromClass "/Game/MyContent/Blueprints/Projectiles/BP_BaseProjectile.BP_BaseProjectile_C" (Math|Transform|MakeTransform (Transformation|GetActorLocation) (Transformation|GetActorRotation) "1.000000,1.000000,1.000000") "AlwaysSpawn" 0 0))