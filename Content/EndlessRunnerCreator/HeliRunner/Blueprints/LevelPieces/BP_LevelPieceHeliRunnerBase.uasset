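; Base level piece for HeliRunner that acts as an obstacle and carries a line of currency pickups along a spline.
; Construction places preview meshes at fixed spacing; BeginPlay swaps them for attached, initially disabled pickup actors.
; A coin flip enables or disables the whole set on BeginPlay and whenever the piece goes out of bounds.
; Enabled pickups are repositioned on the spline because enabling resets their location.
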(event EventBeginPlay
  (|CallParentFunction)
  ;[0 0 0] Remove visual representation of pickups used for testing.
  (for _array_element (Variables|Default|GetCoinMeshArray)
    (Components|DestroyComponent _array_element))
  (CallFunction|SpawnNestedPickups)
  (CallFunction|SetNestedPickupsEnabled (CallFunction|ShouldEnableNestedPickups)))

(event EventTick
  (params (DeltaSeconds :type Float%20%28single-precision%29))
  (|CallParentFunction DeltaSeconds))

(fn ConstructionScript
  (|CallParentFunction)
  (CallFunction|VisualiseNestedPickups))

(fn VisualiseNestedPickups
  (Utilities|Array|Clear (Variables|Default|GetCoinMeshArray))
  (for _index (range 0 (Math|Float|Truncate (/ (Spline|GetSplineLength (Variables|Default|GetSpline)) (Variables|Default|GetNestedPickupSpacing))))
    (LocalVariables|SetCurrentSplinePoint _index)
    ;[0 0 0] These meshes will appear in the wrong place if viewed in the game Map. But line up where intended in the Viewport inside this BP.
    ;
    ; This is working as intended. See comments to the left. These will be removed on BeginPlay and the real Pickups will be spawned in the correct place.
    (bind _returnvalue (AddComponent|AddStaticMeshComponent false (Math|Transform|MakeTransform (.Location (CallFunction|ReturnSplineLocationRotationatPoint (LocalVariables|GetCurrentSplinePoint))) (.Rotation (CallFunction|ReturnSplineLocationRotationatPoint (LocalVariables|GetCurrentSplinePoint))) "1.000000,1.000000,1.000000")))
    (Utilities|Array|Add (Variables|Default|GetCoinMeshArray) _returnvalue)))

(fn SpawnNestedPickups
  ;[0 0 0] Divide the spline by Spacing to define how many pickups to Spawn. Lower Spacing == More Pickups
  (for _index (range 0 (Math|Float|Truncate (/ (Spline|GetSplineLength (Variables|Default|GetSpline)) (Variables|Default|GetNestedPickupSpacing))))
    (LocalVariables|SetCurrentSplinePoint _index)
    ;[0 0 0] Spawn Pickup and attach it to follow this Actor
    (bind _returnvalue (Game|SpawnActorfromClass "/Game/EndlessRunnerCreator/CommonAssets/Blueprints/Spawning/Pickups/BP_SpawnablePickupCurrency.BP_SpawnablePickupCurrency_C" (Math|Transform|MakeTransform (.Location (CallFunction|ReturnSplineLocationRotationatPoint (LocalVariables|GetCurrentSplinePoint))) (.Rotation (CallFunction|ReturnSplineLocationRotationatPoint (LocalVariables|GetCurrentSplinePoint))) "1.000000,1.000000,1.000000") "Undefined" 0 true false 0))
    (bind _output_get (LocalVariables|SetCurrentPickup _returnvalue))
    (Transformation|AttachActorToActor _returnvalue self "None" "KeepWorld" "KeepRelative" "KeepRelative" true)
    (Default|CallDisableObject (LocalVariables|GetCurrentPickup))
    (Utilities|Array|Add (Variables|Default|GetNestedPickups) (LocalVariables|GetCurrentPickup))))

(fn ReturnSplineLocationRotationatPoint
  (params (SplinePoint :type Integer))
  (bind _spline (Variables|Default|GetSpline))
  (bind _nestedpickupspacing (Variables|Default|GetNestedPickupSpacing))
  (bind _returnvalue (* SplinePoint _nestedpickupspacing))
  (return (Spline|GetLocationatDistanceAlongSpline _spline _returnvalue "World") (Spline|GetRotationatDistanceAlongSpline _spline _returnvalue "Local")))

(fn ShouldEnableNestedPickups
  (return (Math|Random|RandomBool)))

(fn SetNestedPickupsEnabled
  (params (SetEnabled :type Boolean))
  ;[0 0 0] Foreach Nested Pickup. Set the enabled state through the pickup interface based on bool passed in
  (for (_array_element _array_index) (Variables|Default|GetNestedPickups)
    (LocalVariables|SetCurrentPickup _array_element)
    (LocalVariables|SetCurrentIndex _array_index)
    (if SetEnabled
      (Default|CallEnableObject (LocalVariables|GetCurrentPickup))
      ;[0 0 0] CallEnableObject resets the ActorLocation when called.
      ;
      ; In this one specific case as it's attached to the Spline, we want to override this and set it back to be in place along the spline
      (Transformation|SetActorLocation (LocalVariables|GetCurrentPickup) (.Location (CallFunction|ReturnSplineLocationRotationatPoint (LocalVariables|GetCurrentIndex))) false false)
      (else
        (Default|CallDisableObject (LocalVariables|GetCurrentPickup))))))

(fn ObjectOutOfBounds
  (|CallParentFunction)
  (CallFunction|SetNestedPickupsEnabled (CallFunction|ShouldEnableNestedPickups)))

(fn CallIsObstacle
  ;[0 0 0] This type of level piece should act as an obstacle and override invincibility to avoid player going out of bounds during invincibility duration.
  (return true false))