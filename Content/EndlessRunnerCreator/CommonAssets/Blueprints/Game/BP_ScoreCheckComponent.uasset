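; Score trigger for the endless runner that awards points when the player passes through its box, which is sized in the construction script.
; On overlap it confirms the player through a message call, adds ScoreValue to the game mode's score, plays a sound and locks further scoring.
; CallEnableObject re-arms it, intended to be called by a recyclable parent Actor when enabled; the other recyclable-object calls are stubs.
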(event OnComponentBeginOverlap(Box)
  (params (OverlappedComponent :type Primitive%20Component%20Object%20Reference) (OtherActor :type Actor%20Object%20Reference) (OtherComp :type Primitive%20Component%20Object%20Reference) (OtherBodyIndex :type Integer) (bFromSweep :type Boolean) (SweepResult :type Hit%20Result%20Structure%20%28by%20ref%29))
  ;[0 0 0] Check if the score component has overlapped the player and if so add score.
  (bind _playerhit (Class|BPIPlayer|CallWasPlayerHit(Message) OtherActor))
  (if (and _playerhit (Variables|Default|GetbCanPlayerScore))
    (bind _currentscore (Class|BPIGameMode|CallGetScore(Message) (Game|GetGameMode)))
    (Class|BPIGameMode|CallSetScore(Message) (Game|GetGameMode) (+ _currentscore (Variables|Score|GetScoreValue)))
    ;[0 0 0] Play Score sound effect.
    (Audio|PlaySoundatLocation (Variables|Default|GetScoreSound) (Transformation|GetActorLocation) "0, 0, 0" 1.0 1.0 0.0 0 0 0 0)
    ;[0 0 0] Set this to false when the player has collected the score for passing once to avoid repeat hits when possibly dying at the same time and respawning on the ScoreCheckComponent for example.
    ;
    ; If this is on a Recyclable object the "CallEnableObject" function should be called on this class from the parent Actor when it is Enabled.
    (Variables|Default|SetbCanPlayerScore false)))

(fn ConstructionScript
  (Components|Box|SetBoxExtent (Variables|Default|GetBox) (Variables|BoxExtent|GetBoxExtent) true))

(fn CallDisableObject
  (return false))

(fn CallEnableObject
  (Variables|Default|SetbCanPlayerScore true)
  (return false))

(fn CallGetEnabled
  (return false))

(fn CallHitMagnet
  (return false))

(fn CallMoveObject
  (params (NewTransform :type Transform))
  (return false))

(fn CallObjectOutOfBounds
  (return false))

(fn CallSetEnabled
  (params (bEnabled :type Boolean))
  (return bEnabled))

(fn CallSetParent
  (params (Parent :type BP%20Spawner%20Base%20Object%20Reference))
  (return false))

(fn CallSetSpeedOffset
  (params (SpeedOffset :type Float%20%28double-precision%29))
  (return false))