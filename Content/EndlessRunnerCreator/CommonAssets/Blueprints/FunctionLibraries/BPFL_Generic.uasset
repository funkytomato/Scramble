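; Blueprint function library of shared helpers for the endless runner game types, covering UI colours, material colour schemes and level manager lookup.
; Colour functions map game type, colour scheme plus actor type, or lizard colour to values, pushing material colours into a "Colour" parameter.
; ReturnMaterialInstance creates a dynamic material from the first valid skeletal mesh, flipbook, static mesh or sprite.
; GetLevelManager expects exactly one manager per level, warning only when a GameInstance exists.
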(fn GetGameTypeUIColour
  (params (CurrentGameType :type EGameType%20Enum :default "NewEnumerator0"))
  (bind __gametypeuicolours (LocalVariables|Get_GameTypeUIColours))
  (bind __gametypeuicolours_2 (LocalVariables|Get_GameTypeUIColours))
  (LocalVariables|Set_GameType CurrentGameType)
  (return (Utilities|Select :Index (LocalVariables|Get_GameType) :NewEnumerator1 (Utilities|Struct|MakeSlateColor (.flappyrunneruicolour __gametypeuicolours_2)) :NewEnumerator4 (Utilities|Struct|MakeSlateColor (.helirunneruicolour __gametypeuicolours_2)) :NewEnumerator2 (Utilities|Struct|MakeSlateColor (.lizardrunneruicolour __gametypeuicolours_2)) :NewEnumerator3 (Utilities|Struct|MakeSlateColor (.roadrunneruicolour __gametypeuicolours_2)) :NewEnumerator5 (Utilities|Struct|MakeSlateColor (.sunrunneruicolour __gametypeuicolours_2)) :NewEnumerator6 (Utilities|Struct|MakeSlateColor (.verticalrunneruicolour __gametypeuicolours_2)) :NewEnumerator0 (Utilities|Struct|MakeSlateColor (.voxelrunneruicolour __gametypeuicolours_2))) (Utilities|Select :Index (LocalVariables|Get_GameType) :NewEnumerator1 (.flappyrunneruicolour __gametypeuicolours) :NewEnumerator4 (.helirunneruicolour __gametypeuicolours) :NewEnumerator2 (.lizardrunneruicolour __gametypeuicolours) :NewEnumerator3 (.roadrunneruicolour __gametypeuicolours) :NewEnumerator5 (.sunrunneruicolour __gametypeuicolours) :NewEnumerator6 (.verticalrunneruicolour __gametypeuicolours) :NewEnumerator0 (.voxelrunneruicolour __gametypeuicolours))))

(fn SetColourSchemeBasedActorValues
  (params (MaterialInstanceRef :type Material%20Instance%20Dynamic%20Object%20Reference) (ActorTypeRef :type ESpawnedObjectType%20Enum :default "NewEnumerator0") (ColourScheme :type EColourScheme%20Enum :default "NewEnumerator0"))
  (bind __colourscheme (LocalVariables|Get_ColourScheme))
  (bind _returnvalue (Utilities|Select :Index ColourScheme :NewEnumerator0 (.greenblack __colourscheme) :NewEnumerator5 (.blueorange __colourscheme) :NewEnumerator4 (.blueorangebright __colourscheme) :NewEnumerator3 (.yellows __colourscheme) :NewEnumerator6 (.shadesofgrey __colourscheme) :NewEnumerator7 (.greyboxing __colourscheme)))
  ;[0 0 0] Set the colour of the specified material instance based on the type of actor calling the function and in which gameType it is called from. This is intended to allow quick updates to be made to colour schemes per gameType.
  (Rendering|Material|SetVectorParameterValue MaterialInstanceRef "Colour" (Utilities|Select :Index ActorTypeRef :NewEnumerator0 (.level _returnvalue) :NewEnumerator1 (.obstacle _returnvalue) :NewEnumerator2 (.player _returnvalue)) :!class /Script/Engine.MaterialInstanceDynamic))

(fn GetLevelManager
  (params (WorldContextObjectRef :type Object%20Object%20Reference))
  (bind _outactors (Actor|GetAllActorsOfClass WorldContextObjectRef "/Game/EndlessRunnerCreator/CommonAssets/Blueprints/Game/BP_LevelManagerBase.BP_LevelManagerBase_C"))
  (if (== (Utilities|Array|Length _outactors) 1)
    (LocalVariables|Set_LevelManagerRef (Utilities|Array|Get(acopy) _outactors))
    (else
      ;[0 0 0] Only print this message if in game. GameInstance IsValid check will only be true when the game has launched, not in the editor.
      ; This is a workaround as there's no, "IsInGame" check.
      (Utilities|IsValid (Game|GetGameInstance)
        (:Is%20Valid
          (CallFunction|GeneralWarningMessage WorldContextObjectRef "There should be exactly ONE level manager in each level.")))))
  (return (LocalVariables|Get_LevelManagerRef)))

(fn ReturnMaterialInstance
  (params (SkeletalMesh :type Skeletal%20Mesh%20Component%20Object%20Reference) (PaperFlipbook :type Paper%20Flipbook%20Component%20Object%20Reference) (StaticMesh :type Static%20Mesh%20Component%20Object%20Reference) (PaperSprite :type Paper%20Sprite%20Component%20Object%20Reference) (CallingActor :type Actor%20Object%20Reference))
  (Utilities|FlowControl|Sequence
    (:then_0
      (Utilities|IsValid SkeletalMesh
        (:Is%20Valid
          ;[0 0 0] Account for Actor classes using a skeletal mesh
          (if (!= (Variables|/Script/Engine.SkinnedMeshComponent|GetSkeletalMesh SkeletalMesh) 0)
            (bind _returnvalue (Rendering|Material|CreateDynamicMaterialInstance SkeletalMesh 0 0 "None" :!class /Script/Engine.PrimitiveComponent))
            (bind _output_get (LocalVariables|Set_PlayerMaterialInstance _returnvalue))
            (return _output_get)))))
    (:then_1
      (Utilities|IsValid PaperFlipbook
        (:Is%20Valid
          ;[0 0 0] Account for Actor classes using a flipbook
          (if (!= (Class|PaperFlipbookComponent|GetFlipbook PaperFlipbook) 0)
            (bind _returnvalue_2 (Rendering|Material|CreateDynamicMaterialInstance PaperFlipbook 0 0 "None" :!class /Script/Engine.PrimitiveComponent))
            (bind _output_get_2 (LocalVariables|Set_PlayerMaterialInstance _returnvalue_2))
            (return _output_get_2)))))
    (:then_2
      (Utilities|IsValid StaticMesh
        (:Is%20Valid
          ;[0 0 0] Account for Actor classes using a Static Mesh
          (if (!= (Variables|/Script/Engine.StaticMeshComponent|GetStaticMesh StaticMesh) 0)
            (bind _returnvalue_3 (Rendering|Material|CreateDynamicMaterialInstance StaticMesh 0 0 "None" :!class /Script/Engine.PrimitiveComponent))
            (bind _output_get_3 (LocalVariables|Set_PlayerMaterialInstance _returnvalue_3))
            (return _output_get_3)))))
    (:then_3
      (Utilities|IsValid PaperSprite
        (:Is%20Valid
          ;[0 0 0] Account for Actor classes using a Paper Sprite
          (if (!= (Sprite|GetSprite PaperSprite) 0)
            (bind _returnvalue_4 (Rendering|Material|CreateDynamicMaterialInstance PaperSprite 0 0 "None" :!class /Script/Engine.PrimitiveComponent))
            (bind _output_get_4 (LocalVariables|Set_PlayerMaterialInstance _returnvalue_4))
            (return _output_get_4)))))
    (:then_4
      ;[0 0 0] If no component types are valid provide Error message.
      (CallFunction|GeneralErrorMessage CallingActor (Utilities|String|Append "Unable to find a valid Mesh or Sprite reference. One of these is required for classses to create Material Instance In Object: " (Utilities|GetDisplayName CallingActor)))
      (return 0))))

(fn SetLizardColour
  (params (MaterialInstanceRef :type Material%20Instance%20Dynamic%20Object%20Reference) (CurrentColour :type ELizardCurrentBlockColour%20Enum :default "NewEnumerator0"))
  (bind __colourscheme (LocalVariables|Get_ColourScheme))
  (bind _returnvalue (Utilities|Select :Index CurrentColour :NewEnumerator0 (.lizardorange __colourscheme) :NewEnumerator1 (.lizardblue __colourscheme) :NewEnumerator2 (.lizardgrey __colourscheme)))
  ;[0 0 0] Set the colour of the specified material instance based on the type of actor calling the function and in which gameType it is called from. This is intended to allow quick updates to be made to colour schemes per gameType.
  (Rendering|Material|SetVectorParameterValue MaterialInstanceRef "Colour" _returnvalue :!class /Script/Engine.MaterialInstanceDynamic)
  (return _returnvalue))